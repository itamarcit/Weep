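; BP_LoopPlayerCharacter is the player character for Loop_Idea, handling movement, camera look and door interaction through Enhanced Input.
; BeginPlay adds the input mapping context to the local player subsystem.
; Move input follows control-rotation yaw only, while look input drives controller yaw and pitch.
; Interact toggles the door held in CurrentInteractDoor, which this graph never assigns, or prints a debug message when none is valid.
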(event Input|EnhancedActionEvents|EnhancedInputActionIA_Loop_Move
  (params (ActionValue :type Vector%202D%20Structure) (ElapsedSeconds :type Float%20%28double-precision%29) (TriggeredSeconds :type Float%20%28double-precision%29) (InputAction :type Input%20Action%20Object%20Reference :default "/Game/Loop_Idea/Input/IA_Loop_Move.IA_Loop_Move"))
  (Pawn|Input|AddMovementInput (Math|Vector|GetRightVector (Math|Rotator|MakeRotator 0.0 0.0 (.Yaw (Math|Rotator|BreakRotator (Pawn|GetControlRotation :!class /Script/Engine.Pawn))))) (.x ActionValue) false)
  (Pawn|Input|AddMovementInput (Math|Vector|GetForwardVector (Math|Rotator|MakeRotator 0.0 0.0 (.Yaw (Math|Rotator|BreakRotator (Pawn|GetControlRotation :!class /Script/Engine.Pawn))))) (.y ActionValue) false))

(event Input|EnhancedActionEvents|EnhancedInputActionIA_Loop_Look
  (params (ActionValue :type Vector%202D%20Structure) (ElapsedSeconds :type Float%20%28double-precision%29) (TriggeredSeconds :type Float%20%28double-precision%29) (InputAction :type Input%20Action%20Object%20Reference :default "/Game/Loop_Idea/Input/IA_Loop_Look.IA_Loop_Look"))
  (Pawn|Input|AddControllerYawInput (.x ActionValue))
  (Pawn|Input|AddControllerPitchInput (.y ActionValue)))

(event Input|EnhancedActionEvents|EnhancedInputActionIA_Loop_Interact
  (params (ActionValue :type Boolean) (ElapsedSeconds :type Float%20%28double-precision%29) (TriggeredSeconds :type Float%20%28double-precision%29) (InputAction :type Input%20Action%20Object%20Reference :default "/Game/Loop_Idea/Input/IA_Loop_Interact.IA_Loop_Interact"))
  (bind _currentinteractdoor (Variables|Default|GetCurrentInteractDoor))
  (Utilities|IsValid _currentinteractdoor
    (:Is%20Valid
      (Default|ToggleDoor _currentinteractdoor))
    (:Is%20Not%20Valid
      (Development|PrintString "No door nearby"))))

(event EventBeginPlay
  (bind _asplayer_controller (Utilities|Casting|CastToPlayerController (Pawn|GetController)))
  (Input|AddMappingContext (PlayerController|LocalPlayerSubsystems|GetEnhancedInputLocalPlayerSubsystem _asplayer_controller) (Variables|Default|GetInputMappingContext) 0 "(bIgnoreAllPressedKeysUntilRelease=True,bForceImmediately=False,bNotifyUserSettings=False)"))

(fn ConstructionScript)