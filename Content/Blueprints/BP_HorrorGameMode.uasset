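; Horror game mode that randomizes the player's start and places the weeping statue far away from it on BeginPlay.
; It teleports the player to a random actor tagged PlayerSpawn, then scans StatueSpawn-tagged actors for the one farthest from that point.
; The first BP_WeepingStatue found in the level is teleported there, with a debug print if none exists.
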(event EventBeginPlay
  (bind _outactors (Actor|GetAllActorswithTag "PlayerSpawn"))
  (if (> (Utilities|Array|Length _outactors) 0)
    (bind _output_get (Variables|Default|SetSelectedPlayerSpawn (Utilities|Array|Get(acopy) _outactors (Math|Random|RandomIntegerinRange 0 (- (Utilities|Array|Length _outactors) 1)))))
    (Transformation|SetActorTransform (Game|GetPlayerCharacter 0) (Transformation|GetActorTransform _output_get) false true)
    (bind _outactors_2 (Actor|GetAllActorswithTag "StatueSpawn"))
    (Variables|Default|SetBestDistance -1.0)
    (Variables|Default|SetBestStatueSpawn 0)
    (for _array_element _outactors_2
      (if (> (Transformation|GetDistanceTo _array_element (Variables|Default|GetSelectedPlayerSpawn)) (Variables|Default|GetBestDistance))
        (Variables|Default|SetBestDistance (Transformation|GetDistanceTo _array_element (Variables|Default|GetSelectedPlayerSpawn)))
        (Variables|Default|SetBestStatueSpawn _array_element)))
    (Utilities|IsValid (Variables|Default|GetBestStatueSpawn)
      (:Is%20Valid
        (bind _outactors_3 (Actor|GetAllActorsOfClass "/Game/Blueprints/BP_WeepingStatue.BP_WeepingStatue_C"))
        (if (> (Utilities|Array|Length _outactors_3) 0)
          (Transformation|SetActorTransform (Utilities|Array|Get(acopy) _outactors_3) (Transformation|GetActorTransform (Variables|Default|GetBestStatueSpawn)) false true)
          (else
            (Development|PrintString "NO STATUE FOUND!!!")))))))

(fn ConstructionScript)