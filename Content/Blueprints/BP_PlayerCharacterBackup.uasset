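; First-person style player character with stamina-limited sprinting and a forced-blink eye meter, both shown on a HUD.
; Tick updates speed and stamina, then drains the eye meter; at zero, a timed camera fade blacks out the view, sets IsBlinking and refills it.
; Holding eyes open pauses drain for a limited time, but adds faster strain drain and a blink-counted cooldown.
; HoldEyesOpen has two overlapping sets of input handlers.
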(event Custom|StartBlink
  (if (not (Variables|Default|GetBlinkInProgress))
    (Variables|Default|SetBlinkInProgress true)
    (Variables|Default|SetWantsToHoldEyesOpen false)
    (Variables|Default|SetEyeHoldActive false)
    (CameraFades|StartCameraFade (Game|GetPlayerCameraManager 0) 0.0 1.0 (Variables|Default|GetBlinkFadeDuration) "(R=0.000000,G=0.000000,B=0.000000,A=1.000000)" false true)
    (Utilities|FlowControl|Delay (Variables|Default|GetBlinkFadeDuration))
    (Variables|Default|SetbIsBlinking true)
    (Utilities|FlowControl|Delay (Variables|Default|GetBlinkDuration))
    (Variables|Default|SetbIsBlinking false)
    (Variables|Default|SetEyeMeter (Variables|Default|GetMaxEyeMeter))
    (Variables|Default|SetCurrentBlinkHoldTime 0.0)
    (Variables|Default|SetEyeStrainActive (Variables|Default|GetEyeStrainNextCycle))
    (Variables|Default|SetEyeStrainNextCycle false)
    (CallFunction|UpdateEyeUI)
    (if (> (Variables|Default|GetEyeHoldCooldownCycles) 0)
      (Variables|Default|SetEyeHoldCooldownCycles (- (Variables|Default|GetEyeHoldCooldownCycles) 1)))
    (Utilities|FlowControl|Delay (Variables|Default|GetBlinkRecoveryDelay))
    (CameraFades|StartCameraFade :self (Game|GetPlayerCameraManager 0) :FromAlpha 1.0 :Duration (Variables|Default|GetBlinkFadeDuration))
    (Utilities|FlowControl|Delay (Variables|Default|GetBlinkFadeDuration))
    (Variables|Default|SetBlinkInProgress false)))

(event Custom|UpdateStaminaUI
  (bind _playerhud (Variables|Default|GetPlayerHUD))
  (Utilities|IsValid _playerhud
    (:Is%20Valid
      (Progress|SetPercent (Variables|/Game/Blueprints/UI/WBP_PlayerHUD.WBP_PlayerHUD_C|GetStaminaBar _playerhud) (/ (Variables|Default|GetSprintStamina) (Variables|Default|GetMaxSprintStamina))))))

(event Custom|UpdateEyeUI
  (bind _playerhud (Variables|Default|GetPlayerHUD))
  (Utilities|IsValid _playerhud
    (:Is%20Valid
      (Progress|SetPercent (Variables|/Game/Blueprints/UI/WBP_PlayerHUD.WBP_PlayerHUD_C|GetEyeBar _playerhud) (/ (Variables|Default|GetEyeMeter) (Variables|Default|GetMaxEyeMeter))))))

(event Custom|UpdateEyeMeter
  (params (DeltaTime :type Float%20%28double-precision%29))
  (if (not (Variables|Default|GetBlinkInProgress))
    (if (and (Variables|Default|GetEyeHoldActive) (< (Variables|Default|GetCurrentBlinkHoldTime) (Variables|Default|GetMaxBlinkHoldTime)))
      (Variables|Default|SetCurrentBlinkHoldTime (+ (Variables|Default|GetCurrentBlinkHoldTime) DeltaTime))
      (elif (Variables|Default|GetEyeStrainActive)
        (Variables|Default|SetEyeMeter (Math|Float|Clamp(Float) (- (Variables|Default|GetEyeMeter) (* (* DeltaTime (Variables|Default|GetEyeDrainRate)) (Variables|Default|GetEyeStrainDrainMultiplier))) 0.0 (Variables|Default|GetMaxEyeMeter)))
        (CallFunction|UpdateEyeUI)
        (if (<= (Variables|Default|GetEyeMeter) 0.0)
          (CallFunction|StartBlink))
        (else
          (Variables|Default|SetEyeMeter (Math|Float|Clamp(Float) (- (Variables|Default|GetEyeMeter) (* (Variables|Default|GetEyeDrainRate) DeltaTime)) 0.0 (Variables|Default|GetMaxEyeMeter)))
          (CallFunction|UpdateEyeUI)
          (if (<= (Variables|Default|GetEyeMeter) 0.0)
            (CallFunction|StartBlink)))))))

(event EventBeginPlay
  ;[0.15 0.15 0.15 0.5] Begin Play
  (bind _returnvalue (UserInterface|CreateWidget "/Game/Blueprints/UI/WBP_PlayerHUD.WBP_PlayerHUD_C"))
  (bind _output_get (Variables|Default|SetPlayerHUD _returnvalue))
  (UserInterface|Viewport|AddtoViewport _output_get 0)
  (Variables|Default|SetSprintStamina (Variables|Default|GetMaxSprintStamina))
  (Variables|/Script/Engine.CharacterMovementComponent|SetMaxWalkSpeed (Variables|Character|GetCharacterMovement) (Variables|Default|GetWalkSpeed))
  (Variables|Default|SetEyeMeter (Variables|Default|GetMaxEyeMeter))
  (CallFunction|UpdateEyeUI)
  (Variables|Default|SetCurrentBlinkHoldTime 0.0)
  (Variables|Default|SetBlinkInProgress false)
  (Variables|Default|SetEyeStrainActive false)
  (Variables|Default|SetEyeStrainNextCycle false)
  (Variables|Default|SetCanUseEyeHold true)
  (Variables|Default|SetEyeHoldCooldownPending false)
  (Variables|Default|SetWantsToHoldEyesOpen false)
  (Variables|Default|SetEyeHoldCooldownCycles 0)
  (Variables|Default|SetEyeHoldActive false))

(event EventTick
  (params (DeltaSeconds :type Float%20%28single-precision%29))
  (Utilities|FlowControl|Sequence
    (:then_0
      (if (and (Variables|Default|GetWantsToSprint) (> (Variables|Default|GetSprintStamina) 0.0))
        (Variables|/Script/Engine.CharacterMovementComponent|SetMaxWalkSpeed (Variables|Character|GetCharacterMovement) (Variables|Default|GetSprintSpeed))
        (Variables|Default|SetSprintStamina (Math|Float|Clamp(Float) (- (Variables|Default|GetSprintStamina) (* (Variables|Default|GetStaminaDrainRate) DeltaSeconds)) 0.0 (Variables|Default|GetMaxSprintStamina)))
        (CallFunction|UpdateStaminaUI)
        (else
          (Variables|/Script/Engine.CharacterMovementComponent|SetMaxWalkSpeed (Variables|Character|GetCharacterMovement) (Variables|Default|GetWalkSpeed))
          (Variables|Default|SetSprintStamina (Math|Float|Clamp(Float) (+ (* DeltaSeconds (Variables|Default|GetStaminaRegenRate)) (Variables|Default|GetSprintStamina)) 0.0 (Variables|Default|GetMaxSprintStamina)))
          (CallFunction|UpdateStaminaUI))))
    (:then_1
      (CallFunction|UpdateEyeMeter DeltaSeconds))))

(event Input|ActionEvents|InputActionSprint
  (params (Key :type Key%20Structure :default "None"))
  ;[0.15 0.15 0.15 0.5] Movement
  (:Pressed
    (Variables|Default|SetWantsToSprint true))
  (:Released
    (Variables|Default|SetWantsToSprint false)))

(event Input|ActionEvents|InputActionHoldEyesOpen
  (params (Key :type Key%20Structure :default "None"))
  ;[0.15 0.15 0.15 0.5] Movement
  (:Pressed
    (Variables|Default|SetWantsToHoldEyesOpen true))
  (:Released
    (Variables|Default|SetWantsToHoldEyesOpen false)
    (if (and (<= (Variables|Default|GetEyeMeter) 0.0) (not (Variables|Default|GetBlinkInProgress)))
      (CallFunction|StartBlink))))

(event Input|ActionEvents|InputActionHoldEyesOpen
  (params (Key :type Key%20Structure :default "None"))
  ;[0.15 0.15 0.15 0.5] Movement
  (:Pressed
    (if (<= (Variables|Default|GetEyeHoldCooldownCycles) 0)
      (Variables|Default|SetWantsToHoldEyesOpen true)
      (Variables|Default|SetEyeHoldActive true)
      (Variables|Default|SetEyeHoldCooldownCycles 2)
      (Variables|Default|SetEyeStrainActive true)
      (Variables|Default|SetEyeStrainNextCycle true)))
  (:Released
    (Variables|Default|SetWantsToHoldEyesOpen false)
    (Variables|Default|SetEyeHoldActive false)))

(event Input|AxisEvents|InputAxisMoveForward
  (params (AxisValue :type Float%20%28single-precision%29))
  ;[0.15 0.15 0.15 0.5] Movement
  (Pawn|Input|AddMovementInput (Transformation|GetActorForwardVector) AxisValue false))

(event Input|AxisEvents|InputAxisMoveRight
  (params (AxisValue :type Float%20%28single-precision%29))
  ;[0.15 0.15 0.15 0.5] Movement
  (Pawn|Input|AddMovementInput (Transformation|GetActorRightVector) AxisValue false))

(event Input|AxisEvents|InputAxisTurn
  (params (AxisValue :type Float%20%28single-precision%29))
  ;[0.15 0.15 0.15 0.5] Movement
  (Pawn|Input|AddControllerYawInput AxisValue))

(event Input|AxisEvents|InputAxisLookUp
  (params (AxisValue :type Float%20%28single-precision%29))
  ;[0.15 0.15 0.15 0.5] Movement
  (Pawn|Input|AddControllerPitchInput AxisValue))

(fn ConstructionScript)