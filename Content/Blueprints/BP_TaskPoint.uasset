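; BP_TaskPoint is a world task point that the player completes by holding interact while in range and looking at it.
; InteractionZone overlaps set range and toggle the progress widget, while StartTask and StopTask set the hold state.
; Tick gates progress with a camera-forward dot product against TaskMesh and updates WBP_TaskProgress.
; Progress persists through interruptions; completion locks the task and only prints a message.
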(event OnComponentBeginOverlap(InteractionZone)
  (params (OverlappedComponent :type Primitive%20Component%20Object%20Reference) (OtherActor :type Actor%20Object%20Reference) (OtherComp :type Primitive%20Component%20Object%20Reference) (OtherBodyIndex :type Integer) (bFromSweep :type Boolean) (SweepResult :type Hit%20Result%20Structure%20%28by%20ref%29))
  (bind _asbp_player_character (Utilities|Casting|CastToBP_PlayerCharacter OtherActor))
  (Variables|Default|SetPlayerCharacter _asbp_player_character)
  (Variables|Default|SetbPlayerInRange true)
  (Development|SetHiddeninGame (Variables|Default|GetProgressWidget) false false))

(event OnComponentEndOverlap(InteractionZone)
  (params (OverlappedComponent :type Primitive%20Component%20Object%20Reference) (OtherActor :type Actor%20Object%20Reference) (OtherComp :type Primitive%20Component%20Object%20Reference) (OtherBodyIndex :type Integer))
  (Utilities|Casting|CastToBP_PlayerCharacter OtherActor)
  (Variables|Default|SetbPlayerInRange false)
  (Variables|Default|SetbPlayerHoldingInteract false)
  (Development|SetHiddeninGame (Variables|Default|GetProgressWidget) true false))

(event Custom|StartTask
  (if (not (Variables|Default|GetbIsCompleted))
    (Variables|Default|SetbPlayerHoldingInteract true)))

(event Custom|StopTask
  (Variables|Default|SetbPlayerHoldingInteract false))

(event EventTick
  (params (DeltaSeconds :type Float%20%28single-precision%29))
  (bind _returnvalue (Game|GetPlayerCameraManager 0))
  (if (and (and (Variables|Default|GetbPlayerInRange) (Variables|Default|GetbPlayerHoldingInteract)) (not (Variables|Default|GetbIsCompleted)))
    (if (> (Math|Vector|DotProduct (Math|Vector|Normalize (- (Transformation|GetWorldLocation (Variables|Default|GetTaskMesh)) (Camera|GetCameraLocation _returnvalue))) (Math|Vector|GetForwardVector (Camera|GetCameraRotation _returnvalue))) (Variables|Default|GetLookDotThreshold))
      (Variables|Default|SetCurrentProgress (Math|Float|Clamp(Float) (+ (Variables|Default|GetCurrentProgress) DeltaSeconds) 0.0 (Variables|Default|GetTaskTimeRequired)))
      (bind _aswbp_task_progress (Utilities|Casting|CastToWBP_TaskProgress (UserInterface|GetUserWidgetObject (Variables|Default|GetProgressWidget))))
      (Progress|SetPercent (Variables|/Game/Blueprints/UI/WBP_TaskProgress.WBP_TaskProgress_C|GetProgressBar_Task _aswbp_task_progress) (/ (Variables|Default|GetCurrentProgress) (Variables|Default|GetTaskTimeRequired)))
      (if (>= (Variables|Default|GetCurrentProgress) (Variables|Default|GetTaskTimeRequired))
        (Variables|Default|SetbIsCompleted true)
        (Variables|Default|SetbPlayerHoldingInteract false)
        (Development|PrintString "Task Completed")))))

(fn ConstructionScript)