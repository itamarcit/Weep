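; BP_TaskManager tracks task completion in a level with weeping statue enemies and escalates difficulty as tasks finish.
; On BeginPlay it counts task points, caches the player and existing statues, and initializes the task counter UI.
; Each registered completion updates the UI, raises entity speed by tier and, at later tiers, spawns entities at random tagged points.
; Completing all tasks stops player input and fades out the camera.
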(event Custom|RegisterTaskCompleted
  (bind _playercharacter (Variables|Default|GetPlayerCharacter))
  (Variables|Default|SetCompletedTasks (+ (Variables|Default|GetCompletedTasks) 1))
  (Utilities|IsValid _playercharacter
    (:Is%20Valid
      (Default|UpdateTaskCounterUI _playercharacter (Variables|Default|GetCompletedTasks) (Variables|Default|GetTotalTasks))
      (CallFunction|ApplyDifficulty))
    (:Is%20Not%20Valid
      (CallFunction|ApplyDifficulty)))
  (if (>= (Variables|Default|GetCompletedTasks) (Variables|Default|GetTotalTasks))
    (CallFunction|FinishLevel)))

(event Custom|ApplyDifficulty
  (switch int (Variables|Default|GetCompletedTasks)
    (:0
      (CallFunction|SetAllEntitySpeeds 2.5e+02))
    (:1
      (CallFunction|SetAllEntitySpeeds 3.2e+02))
    (:2
      (CallFunction|SetAllEntitySpeeds 4e+02))
    (:3
      (CallFunction|SpawnEntityifNeeded 2)
      (CallFunction|SetAllEntitySpeeds 4.6e+02))
    (:4
      (CallFunction|SpawnEntityifNeeded 3)
      (CallFunction|SetAllEntitySpeeds 5.3e+02))))

(event Custom|FinishLevel
  (bind _returnvalue (Game|GetPlayerController 0))
  (Development|PrintString "LEVEL COMPLETE")
  (Input|SetIgnoreMoveInput _returnvalue true)
  (Input|SetIgnoreLookInput _returnvalue true)
  (Components|Movement|StopMovementImmediately (Variables|/Script/Engine.Character|GetCharacterMovement (Game|GetPlayerCharacter 0)))
  (CameraFades|StartCameraFade :self (Game|GetPlayerCameraManager 0) :ToAlpha 1.0 :Duration 2.0 :bShouldFadeAudio true :bHoldWhenFinished true))

(event Custom|SetAllEntitySpeeds
  (params (NewSpeed :type Float%20%28double-precision%29))
  (for _array_element (Variables|Default|GetEntityRefs)
    (Utilities|IsValid _array_element
      (:Is%20Valid
        (Default|SetEntitySpeed _array_element NewSpeed)
        (Development|PrintString "ENTITY SPEED UPDATED")))))

(event Custom|SpawnEntityIfNeeded
  (params (TargetEntityCount :type Integer))
  (if (< (Utilities|Array|Length (Variables|Default|GetEntityRefs)) TargetEntityCount)
    (CallFunction|SpawnOneEntity)))

(event Custom|SpawnOneEntity
  (bind _outactors (Actor|GetAllActorswithTag "StatueSpawn"))
  (if (> (Utilities|Array|Length _outactors) 0)
    (bind _returnvalue (Game|SpawnActorfromClass (Variables|Default|GetEntityClass) (Transformation|GetActorTransform (Utilities|Array|Get(acopy) _outactors (Math|Random|RandomIntegerinRange 0 (- (Utilities|Array|Length _outactors) 1)))) "AlwaysSpawn" "MultiplyWithRoot" 0 0))
    (Utilities|IsValid _returnvalue
      (:Is%20Valid
        (Utilities|Array|Add (Variables|Default|GetEntityRefs) _returnvalue)
        (Development|PrintString "NEW ENTITY SPAWNED")))))

(event EventBeginPlay
  (Utilities|FlowControl|Delay 0.2)
  (bind _outactors (Actor|GetAllActorsOfClass "/Game/Blueprints/BP_TaskPoint.BP_TaskPoint_C"))
  (Variables|Default|SetTotalTasks (Utilities|Array|Length _outactors))
  (bind _asbp_player_character (Utilities|Casting|CastToBP_PlayerCharacter (Game|GetPlayerCharacter 0)))
  (bind _output_get (Variables|Default|SetPlayerCharacter _asbp_player_character))
  (Default|UpdateTaskCounterUI _output_get (Variables|Default|GetCompletedTasks) (Variables|Default|GetTotalTasks))
  (bind _outactors_2 (Actor|GetAllActorsOfClass "/Game/Blueprints/BP_WeepingStatue.BP_WeepingStatue_C"))
  (Variables|Default|SetEntityRefs _outactors_2))

(fn ConstructionScript)