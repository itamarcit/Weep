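; BP_WeepingStatue is a weeping-angel style enemy that creeps toward the player whenever unobserved and triggers a jumpscare on reaching catch distance.
; A looping timer checks the player's blink state, a camera dot product and a visibility trace, then either freezes movement and animation or issues AI MoveTo.
; Each tick of that timer also scales presence and movement audio volume by distance to the player.
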(event Custom|UpdateStatueLogic
  (bind _playercharacter (Variables|Default|GetPlayerCharacter))
  (bind _playercamera (Variables|/Game/Blueprints/BP_PlayerCharacter.BP_PlayerCharacter_C|GetPlayerCamera _playercharacter))
  (CallFunction|UpdateEntityAudio)
  (Utilities|IsValid _playercharacter
    (:Is%20Valid
      (CallFunction|CheckCaughtPlayer)
      (if (not (Variables|Default|GetbHasCaughtPlayer))
        (if (Variables|/Game/Blueprints/BP_PlayerCharacter.BP_PlayerCharacter_C|GetbIsBlinking (Variables|Default|GetPlayerCharacter))
          (CallFunction|MoveTowardPlayer)
          (elif (> (Math|Vector|DotProduct (Math|Vector|Normalize (- (Transformation|GetActorLocation) (Transformation|GetWorldLocation _playercamera))) (Math|Vector|GetForwardVector (Transformation|GetWorldRotation _playercamera))) (Variables|Default|GetLookDotThreshold))
            (bind _outhit (Collision|LineTraceByChannel (Transformation|GetWorldLocation (Variables|/Game/Blueprints/BP_PlayerCharacter.BP_PlayerCharacter_C|GetPlayerCamera (Variables|Default|GetPlayerCharacter))) (+ (Transformation|GetActorLocation) "0.000000,0.000000,60.000000") "TraceTypeQuery1" false 0 "None" false))
            (if (== (.HitActor (Collision|BreakHitResult _outhit)) self)
              (CallFunction|FreezeStatue)
              (else
                (CallFunction|MoveTowardPlayer)))
            (else
              (CallFunction|MoveTowardPlayer))))))))

(event Custom|FreezeStatue
  (CallFunction|StopEntityMovementSound)
  (Variables|/Script/Engine.CharacterMovementComponent|SetMaxWalkSpeed (Variables|Character|GetCharacterMovement) 0.0)
  (Components|Movement|StopMovementImmediately (Variables|Character|GetCharacterMovement))
  (Variables|/Script/Engine.SkeletalMeshComponent|SetGlobalAnimRateScale (Variables|Character|GetMesh) 0.0))

(event Custom|MoveTowardPlayer
  (CallFunction|StartEntityMovementSound)
  (Variables|/Script/Engine.CharacterMovementComponent|SetMaxWalkSpeed (Variables|Character|GetCharacterMovement) (Variables|Default|GetMoveSpeed))
  (Variables|/Script/Engine.SkeletalMeshComponent|SetGlobalAnimRateScale (Variables|Character|GetMesh) 0.75)
  (AI|AIMoveTo self (Transformation|GetActorLocation (Variables|Default|GetPlayerCharacter)) 0 (Variables|Default|GetStopDistance) true))

(event Custom|CheckCaughtPlayer
  (if (not (Variables|Default|GetbHasCaughtPlayer))
    (if (< (Transformation|GetDistanceTo (Variables|Default|GetPlayerCharacter)) (Variables|Default|GetCatchDistance))
      (Variables|Default|SetbHasCaughtPlayer true)
      (CallFunction|StopEntityMovementSound)
      (Default|TriggerJumpscare (Variables|Default|GetPlayerCharacter))
      (CallFunction|FreezeStatue)
      (Utilities|FlowControl|Delay 1.0))))

(event Custom|StartEntityMovementSound
  (bind _entitymovementaudio (Variables|Default|GetEntityMovementAudio))
  (if (not (Audio|Components|Audio|IsPlaying _entitymovementaudio))
    (CallFunction|UpdateEntityAudio)
    (Audio|Components|Audio|Play _entitymovementaudio 0.0)))

(event Custom|StopEntityMovementSound
  (bind _entitymovementaudio (Variables|Default|GetEntityMovementAudio))
  (if (Audio|Components|Audio|IsPlaying _entitymovementaudio)
    (Audio|Components|Audio|FadeOut _entitymovementaudio 0.15 0.0 "Linear" :!class /Script/Engine.AudioComponent)))

(event Custom|UpdateEntityAudio
  (bind _playercharacter (Variables|Default|GetPlayerCharacter))
  (Utilities|IsValid _playercharacter
    (:Is%20Valid
      (Variables|Default|SetEntityAudioAmount (Math|Float|MapRangeClamped (Transformation|GetDistanceTo _playercharacter) (Variables|Default|GetEntityAudioMaxDistance) (Variables|Default|GetEntityAudioMinDistance) 0.0 1.0))
      (Audio|Components|Audio|SetVolumeMultiplier (Variables|Default|GetEntityPresenceAudio) (Math|Float|Lerp 0.0 (Variables|Default|GetEntityPresenceMaxVolume) (Variables|Default|GetEntityAudioAmount)) :!class /Script/Engine.AudioComponent)
      (Audio|Components|Audio|SetVolumeMultiplier (Variables|Default|GetEntityMovementAudio) (Math|Float|Lerp 0.0 (Variables|Default|GetEntityPresenceMaxVolume) (Variables|Default|GetEntityAudioAmount)) :!class /Script/Engine.AudioComponent))))

(event Custom|SetEntitySpeed
  (params (NewSpeed :type Float%20%28double-precision%29))
  (Variables|Default|SetMoveSpeed NewSpeed))

(event EventBeginPlay
  (bind _asbp_player_character (Utilities|Casting|CastToBP_PlayerCharacter (Game|GetPlayerCharacter 0)))
  (Variables|Default|SetPlayerCharacter _asbp_player_character)
  (Utilities|FlowControl|Delay 0.2)
  (Utilities|Time|SetTimerbyEvent (delegate Custom|UpdateStatueLogic) (Variables|Default|GetCheckInterval) true))

(fn ConstructionScript)